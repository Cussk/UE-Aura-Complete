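; Gameplay ability for enemy melee attacks that turns toward the combat target, then plays a random tagged montage from the avatar.
; A montage gameplay event triggers a small sphere check at the attack's weapon socket, damaging non-allied live characters.
; On a hit it executes one melee impact gameplay cue, passing montage tag, location and target.
; The ability ends after that check, while the montage keeps playing, or when the montage finishes or is interrupted.
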(event Ability|EventActivateAbility
  (bind _returnvalue (Ability|GetAvatarActorfromActorInfo))
  (CallFunction|UpdateMotionWarpingRotation)
  ;[0.0865 1 0 0.502] Get all the FTaggedMontages structs from the owning actor.  Get a random Attack from the array.
  (bind _returnvalue_2 (Class|CombatInterface|GetAttackMontages(Message) (Ability|GetAvatarActorfromActorInfo)))
  (bind _output_get (Variables|Default|SetTaggedMontage (.OutItem (Utilities|Array|Random _returnvalue_2))))
  ;[0.0865 1 0 0.502] Play the attack montage and wait for the corresponding GameplayTag notify to be called from the montage
  (|PlayMontageandWaitProxy "None" (.Montage (Utilities|Struct|BreakTaggedMontage _output_get)) 1.0 "None" false 1.0 0.0 false
    (:then
      (Ability|Tasks|WaitGameplayEvent (.MontageTag (Utilities|Struct|BreakTaggedMontage (Variables|Default|GetTaggedMontage))) 0
        (:EventReceived
          ;[0.0865 1 0 0.502] Get the montage tag that matches the attacking weapon socket
          (bind _returnvalue_3 (Class|CombatInterface|GetCombatSocketLocation(Message) _returnvalue (.SocketTag (Utilities|Struct|BreakTaggedMontage (Variables|Default|GetTaggedMontage)))))
          (CallFunction|DamageEnemiesinRange self (Utilities|Array|MakeArray _returnvalue) _returnvalue_3))))
    (:OnCompleted
      (Ability|EndAbility :!label _label))
    (:OnInterrupted
      (goto _label))
    (:OnCancelled
      (goto _label))))

(fn UpdateMotionWarpingRotation
  (bind _returnvalue (Ability|GetAvatarActorfromActorInfo))
  (bind _returnvalue_2 (Class|TargetInterface|GetCombatTarget(Message) _returnvalue))
  (Class|CombatInterface|UpdateFacingTarget(Message) _returnvalue (Transformation|GetActorLocation _returnvalue_2)))

(fn DamageEnemiesinRange
  (params (WorldContextObject :type Object%20Object%20Reference) (ActorsToIgnore :type Array%20of%20Actor%20Object%20References) (SphereOrigin :type Vector%20%28by%20ref%29))
  (LocalVariables|SetCombatSocketLocation SphereOrigin)
  (Variables|Default|SetbHasHitTarget false)
  (bind _outoverlappingactors (Class|AuraAbilitySystemLibrary|GetLivePlayersWithinRadius WorldContextObject ActorsToIgnore 45.0 (LocalVariables|GetCombatSocketLocation)))
  ;[0.0865 1 0 0.502] Loop through characters found in radius, check actors for matching "Player" or "Enemy" tags, cause damage if they don't match
  (for _array_element _outoverlappingactors
    (if (not (Class|AuraAbilitySystemLibrary|IsAlly (Ability|GetAvatarActorfromActorInfo) _array_element))
      (Class|AuraDamageGameplayAbility|CauseDamage _array_element)
      (Variables|Default|SetbHasHitTarget true)))
  (CallFunction|TryFireGameplayCue (LocalVariables|GetCombatSocketLocation)))

(fn TryFireGameplayCue
  (params (CombatSocketLocation :type Vector))
  ;[0.0865 1 0 0.502] Fire Gameplay Cue for impact effects once after loop only if target hit.  Populate Gameplay Cue Parameters with Montage Tag, Combat Socket Location, Target Actor, and Owner Actor
  (if (Variables|Default|GetbHasHitTarget)
    (bind _returnvalue (Class|TargetInterface|GetCombatTarget(Message) (Ability|GetAvatarActorfromActorInfo)))
    (Class|GameplayAbility|ExecuteGameplayCuewithParams "(TagName=\"GameplayCue.MeleeImpact\")" (Ability|GameplayCue|MakeGameplayCueParameters :AggregatedSourceTags (GameplayTags|MakeGameplayTagContainerfromTag (.MontageTag (Utilities|Struct|BreakTaggedMontage (Variables|Default|GetTaggedMontage)))) :Location CombatSocketLocation :EffectCauser (Ability|GetAvatarActorfromActorInfo) :SourceObject _returnvalue))
    (Ability|EndAbility)
    (else
      (Ability|EndAbility))))