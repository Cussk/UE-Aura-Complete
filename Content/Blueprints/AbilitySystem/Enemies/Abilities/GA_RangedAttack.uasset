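; Enemy ranged attack gameplay ability that plays an attack animation and launches a projectile at the combat target.
; On activation it stores the target's location and updates motion warping facing through combat interface calls on the avatar, then plays a random attack montage.
; The montage's gameplay tag event triggers the projectile spawn from the tagged socket with an overridden pitch.
; The ability ends when the montage completes, is interrupted or is cancelled.
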(event Ability|EventActivateAbility
  (CallFunction|UpdateMotionWarpingRotation)
  (bind _returnvalue (Class|CombatInterface|GetAttackMontages(Message) (Ability|GetAvatarActorfromActorInfo)))
  (bind _output_get (Variables|Default|SetTaggedMontage (.OutItem (Utilities|Array|Random _returnvalue))))
  (|PlayMontageandWaitProxy "None" (.Montage (Utilities|Struct|BreakTaggedMontage _output_get)) 1.0 "None" false 1.0 0.0 false
    (:then
      (Ability|Tasks|WaitGameplayEvent (.MontageTag (Utilities|Struct|BreakTaggedMontage _output_get)) 0
        (:EventReceived
          (Class|AuraProjectileSpell|SpawnProjectile (Variables|Default|GetTargetLocation) (.SocketTag (Utilities|Struct|BreakTaggedMontage _output_get)) true 25.0))))
    (:OnCompleted
      (Ability|EndAbility :!label _label))
    (:OnInterrupted
      (goto _label))
    (:OnCancelled
      (goto _label))))

(fn UpdateMotionWarpingRotation
  (bind _returnvalue (Ability|GetAvatarActorfromActorInfo))
  (bind _returnvalue_2 (Class|TargetInterface|GetCombatTarget(Message) _returnvalue))
  (bind _output_get (Variables|Default|SetTargetLocation (Transformation|GetActorLocation _returnvalue_2)))
  (Class|CombatInterface|UpdateFacingTarget(Message) _returnvalue _output_get))