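; Enemy summon gameplay ability that currently only previews spawn points with debug spheres, without spawning any actors.
; On activation it stores the result of GetSpawnLocations and shuffles the array.
; A Delay-driven loop then steps through the index, drawing one short-lived sphere at a time for a staggered sequence.
; The graph neither resets the index nor calls EndAbility.
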(event Ability|EventActivateAbility
  (bind _returnvalue (Class|AuraSummonAbility|GetSpawnLocations false))
  (bind _output_get (Variables|Default|SetSpawnLocations _returnvalue))
  (Utilities|Array|Shuffle _output_get)
  (if (< (Variables|Default|GetSpawnLocationIndex) (Utilities|Array|Length (Variables|Default|GetSpawnLocations))) :!label _label
    (Rendering|Debug|DrawDebugSphere (Utilities|Array|Get(acopy) (Variables|Default|GetSpawnLocations) (Variables|Default|GetSpawnLocationIndex)) 25.0 12 "(R=1.000000,G=0.000000,B=0.549374,A=1.000000)" 3.0)
    (Math|Integer|IncrementInt (Variables|Default|GetSpawnLocationIndex)
      (:%20%20
        (Utilities|FlowControl|Delay 0.2)
        (goto _label)))))