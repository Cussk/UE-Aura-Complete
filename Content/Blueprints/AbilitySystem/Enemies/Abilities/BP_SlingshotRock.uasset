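; BP_SlingshotRock is the rock used by an enemy slingshot ability, tumbling at random as it exists in the world.
; BeginPlay picks random pitch, yaw and roll rates, which Tick scales by delta time to spin the rock mesh locally.
; Sphere collision switches to query-only after a short delay, so rocks from small characters do not hit the ground on spawn.
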(event EventBeginPlay
  (bind _returnvalue (Math|Random|RandomFloatinRange -5e+02 5e+02))
  ;[0.5156 0.4877 0 0.5] Random Rotation of Rock
  (Variables|Default|SetPitchRotationRate _returnvalue)
  (Variables|Default|SetYawRotationRate _returnvalue)
  (Variables|Default|SetRollRotationRate _returnvalue)
  ;[1 0.7112 0 0.5] Slight delay before activating collision to not collide with ground on small characters
  (Utilities|FlowControl|Delay 0.1)
  (bind _sphere (Variables|Default|GetSphere)
    (:then
      (Collision|SetCollisionEnabled _sphere "QueryOnly"))
    (:else)))

(event EventTick
  (params (DeltaSeconds :type Float%20%28single-precision%29))
  ;[0.5156 0.4877 0 0.5] Random Rotation of Rock
  (Transformation|AddLocalRotation (Variables|Default|GetRockMesh) (Math|Rotator|MakeRotator (* DeltaSeconds (Variables|Default|GetRollRotationRate)) (* DeltaSeconds (Variables|Default|GetPitchRotationRate)) (* DeltaSeconds (Variables|Default|GetYawRotationRate))) false false))

(fn ConstructionScript)